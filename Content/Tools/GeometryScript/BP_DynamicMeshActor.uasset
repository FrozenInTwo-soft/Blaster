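; Base dynamic mesh actor for geometry scripting, whose child classes build the mesh in OnCreateDynamicMesh.
; Construction requests a gated, timer-delayed rebuild scheduled by the generation manager, and BeginPlay closes the gate if runtime rebuilds are disallowed.
; Rebuilds defer collision updates, optionally clear the mesh, boolean-subtract overlapping subtractive actors' components, then reset collision and reopen the gate.
; A helper detects and optionally deletes degenerate triangles.
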(event Custom|RequestDynamicMeshRebuild
  ;[1 1 1] Dynamic Mesh Update
  (Utilities|FlowControl|Gate false
    (:Exit
      (if (not (Variables|DynamicMeshSettings|GetDisableMeshRebuild))
        (CallFunction|DisableDynamicMeshRebuildRequests)
        (bind _returnvalue (Default|GetUpdateWaitTime (CallFunction|GetDynamicMeshGenerationManager) (Utilities|Time|GetGameTimeinSeconds)))
        (Utilities|Time|SetTimerbyFunctionName 0 "RebuildDynamicMesh" _returnvalue)))))

(event Custom|DisableDynamicMeshRebuildRequests
  ;[1 1 1] Dynamic Mesh Update
  (Utilities|FlowControl|Gate false) ; enters at Close
)

(event Custom|EnableDynamicMeshRebuildRequests
  ;[1 1 1] Dynamic Mesh Update
  (Utilities|FlowControl|Gate false) ; enters at Open
)

(event Custom|OnCreateDynamicMesh
  (params (Target :type Dynamic%20Mesh%20Object%20Reference))
  ;[1 0.2338 0.3236] Implement in child class
)

(event EventBeginPlay
  (if (CallFunction|CanRebuildMeshatRuntime)
    (CallFunction|DisableDynamicMeshRebuildRequests)))

(fn ConstructionScript
  (CallFunction|RequestDynamicMeshRebuild))

(fn RebuildDynamicMesh
  (bind _self self)
  (bind _dynamicmeshcomponent (Variables|DynamicMeshActor|GetDynamicMeshComponent))
  (bind _returnvalue (DynamicMeshComponent|GetDynamicMesh (Variables|DynamicMeshActor|GetDynamicMeshComponent)))
  (LocalVariables|SetCurrentDynamicMesh _returnvalue)
  (Utilities|FlowControl|Sequence
    (:then_0
      ;[1 1 1] Automatically defer collision updates during generated mesh rebuild. If we do not do this, then each mesh change will result in collision being rebuilt, which is very expensive !!
      (LocalVariables|SetEnableDeferredCollision false)
      (if (not (Variables|/Script/GeometryFramework.DynamicMeshComponent|GetbDeferCollisionUpdates _dynamicmeshcomponent))
        (Class|DynamicMeshComponent|SetDeferredCollisionUpdatesEnabled _dynamicmeshcomponent true false)
        (LocalVariables|SetEnableDeferredCollision true)))
    (:then_1
      ;[1 1 1] Clear current dynamic mesh if needed
      (if (Variables|DynamicMeshSettings|GetClearMeshOnRebuild)
        (DynamicMesh|Reset (LocalVariables|GetCurrentDynamicMesh))))
    (:then_2
      ;[1 1 1] Create dynamic mesh
      (CallFunction|OnCreateDynamicMesh (LocalVariables|GetCurrentDynamicMesh)))
    (:then_3
      ;[1 1 1] ApplySubtractiveShapes
      (bind _outactors (Actor|GetAllActorsOfClass (CallFunction|GetDynamicSubtractiveActorClass)))
      (for _array_element _outactors
        (if (!= (Actor|GetParentActor _array_element) _self)
          (bind _returnvalue_2 (CallFunction|AreActorsOverlapping _array_element _self false false "0, 0, 0"))
          (if _returnvalue_2
            (bind _asbp_subtractive_geometry_actor (Utilities|Casting|CastToBP_SubtractiveGeometryActor _array_element))
            (bind _return (Default|GetGeometrySubtractiveComponents _asbp_subtractive_geometry_actor))
            (for _array_element_2 _return
              (bind _returnvalue_3 (DynamicMeshActor|AllocateComputeMesh))
              (bind _returnvalue_4 (GeometryScript|Scene|CopyMeshfromComponent :Component _array_element_2 :ToDynamicMesh _returnvalue_3 :bTransformToWorld true :Debug 0)
                (:Success
                  (GeometryScript|Booleans|ApplyMeshBoolean :TargetMesh (LocalVariables|GetCurrentDynamicMesh) :TargetTransform (Transformation|GetActorTransform) :ToolMesh _returnvalue_4 :Operation "Subtract" :Debug 0)))))))
      (Utilities|Array|Clear _outactors)
      (DynamicMeshActor|ReleaseAllComputeMeshes))
    (:then_4
      (if (LocalVariables|GetEnableDeferredCollision)
        (Class|DynamicMeshComponent|SetDeferredCollisionUpdatesEnabled (Variables|DynamicMeshActor|GetDynamicMeshComponent) false false)))
    (:then_5
      (Class|GeometryScriptLibraryCollisionFunctions|ResetDynamicMeshCollision (Variables|DynamicMeshActor|GetDynamicMeshComponent) false 0))
    (:then_6
      (CallFunction|EnableDynamicMeshRebuildRequests))))

(fn CanRebuildMeshatRuntime
  (return (or (not (Variables|DynamicMeshSettings|GetAllowMeshRebuildAtRuntime)) (not (Variables|/Game/Tools/GeometryScript/BP_MeshGenerationManager.BP_MeshGenerationManager_C|GetCanRebuildMeshesAtRuntime (CallFunction|GetDynamicMeshGenerationManager))))))

(fn CleanDegenerateTris
  (params (Mesh :type Dynamic%20Mesh%20Object%20Reference) (SafeNormalTolerance :type Float%20%28double-precision%29) (DebugLogCount :type Boolean) (DeleteDegenerates :type Boolean))
  (bind _triangleidlist (GeometryScript|MeshQueries|GetAllTriangleIDs Mesh))
  (bind _indexarray (Class|GeometryScriptLibraryListUtilityFunctions|ConvertIndexListtoArray _triangleidlist))
  (for _array_element _indexarray
    (Math|Float|CompareFloat (Math|Vector|VectorLengthSquared (Math|Vector|CrossProduct (- (.Vertex3 (Class|GeometryScriptLibraryMeshQueryFunctions|GetTrianglePositions Mesh _array_element)) (.Vertex1 (Class|GeometryScriptLibraryMeshQueryFunctions|GetTrianglePositions Mesh _array_element))) (- (.Vertex2 (Class|GeometryScriptLibraryMeshQueryFunctions|GetTrianglePositions Mesh _array_element)) (.Vertex1 (Class|GeometryScriptLibraryMeshQueryFunctions|GetTrianglePositions Mesh _array_element))))) SafeNormalTolerance
      (:<
        (Utilities|Array|Add (LocalVariables|GetDegenerateTriList) _array_element))))
  (if (not (Utilities|Array|IsEmpty (LocalVariables|GetDegenerateTriList)))
    (Utilities|FlowControl|Sequence
      (:then_0
        (if DebugLogCount
          (Development|PrintString (Utilities|String|Append (Utilities|String|Append (Utilities|String|MakeLiteralString "Found ") (Utilities|String|ToString(Integer) (Utilities|Array|Length (LocalVariables|GetDegenerateTriList)))) (Utilities|String|MakeLiteralString " Degenerates")))))
      (:then_1
        (if DeleteDegenerates
          (bind _indexlist (GeometryScript|ListUtils|ConvertArraytoIndexList (LocalVariables|GetDegenerateTriList) "Triangle"))
          (bind _returnvalue (Class|GeometryScriptLibraryMeshBasicEditFunctions|DeleteTrianglesfromMesh Mesh _indexlist false))
          (Class|GeometryScriptLibraryMeshRepairFunctions|CompactMesh _returnvalue 0))))))