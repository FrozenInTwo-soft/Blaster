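; Mesh generation manager Blueprint for Geometry Script tools that calculates how long to wait before a mesh update.
; By default it returns a short fixed interval.
; When deferred rebuilds are forced, it tracks the last scheduled update time so successive requests queue at increasing delays, staggering them up to a capped maximum wait.
; The schedule resets to the current time if it runs beyond that cap.
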(fn GetUpdateWaitTime
  (params (CurrentGameTime :type Float%20%28double-precision%29))
  (if (Variables|Default|GetForceDeferredMeshesRebuild)
    (Utilities|FlowControl|Sequence
      (:then_0
        (if (> (- (Variables|Hidden|GetLastUpdatedMeshTime) CurrentGameTime) (CallFunction|GetUpdateIntervalMax))
          (Variables|Hidden|SetLastUpdatedMeshTime CurrentGameTime)))
      (:then_1
        (LocalVariables|SetCalculatedUpdateTime (Math|Float|Min(Float) (+ (Math|Float|Max(Float) (- (Variables|Hidden|GetLastUpdatedMeshTime) CurrentGameTime) 0.0) (CallFunction|GetUpdateInterval)) (CallFunction|GetUpdateIntervalMax))))
      (:then_2
        (Variables|Hidden|SetLastUpdatedMeshTime (+ CurrentGameTime (LocalVariables|GetCalculatedUpdateTime))))
      (:then_3
        (return (LocalVariables|GetCalculatedUpdateTime))))
    (else
      (return (CallFunction|GetUpdateInterval)))))

(fn GetUpdateInterval
  (return 0.05))

(fn GetUpdateIntervalMax
  (return 2.0))