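; Base Blueprint for Geometry Script tool actors that supply subtractive geometry to dynamic mesh actors.
; Child classes implement GetGeometrySubtractiveComponents to provide the subtractive components.
; Construction and destruction find dynamic mesh actors overlapping within a padded extent and request their rebuild.
; The construction script rebinds OnDestroyed for this, and BeginPlay unbinds it so destruction during play triggers no rebuild.
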(event EventBeginPlay
  (EventDispatchers|UnbindallEventsfromOnDestroyed))

(event Collision|EventActorBeginOverlap
  (params (OtherActor :type Actor%20Object%20Reference)))

(event EventTick
  (params (DeltaSeconds :type Float%20%28single-precision%29)))

(fn ConstructionScript
  (EventDispatchers|UnbindallEventsfromOnDestroyed)
  (Game|BindEventtoOnDestroyed (EventDispatchers|CreateEvent :!event OnActorDestroyed))
  (CallFunction|RequestOverlappingDynamicMeshesRebuild))

(fn GetGeometrySubtractiveComponents
  ;[1 1 1] Implement in Child Class
  (return 0))

(fn OnActorDestroyed
  (params (DestroyedActor :type Actor%20Object%20Reference))
  (CallFunction|RequestOverlappingDynamicMeshesRebuild))

(fn RequestOverlappingDynamicMeshesRebuild
  (bind _outactors (Actor|GetAllActorsOfClass (CallFunction|GetDynamicMeshActorClass)))
  (for _array_element _outactors
    (bind _returnvalue (CallFunction|AreActorsOverlapping _array_element self false false "200.000000,200.000000,200.000000"))
    (if _returnvalue
      (Default|RequestDynamicMeshRebuild _array_element)))
  (Utilities|Array|Clear _outactors))