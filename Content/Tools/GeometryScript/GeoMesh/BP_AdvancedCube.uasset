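; BP_AdvancedCube is a Geometry Script generated mesh actor that builds a parametric box, solid or hollow.
; On mesh creation it sizes and offsets a box from the Handle vector, applies box-projected UVs and assigns the Material.
; When Hollow is set, it boolean-subtracts an inner box built on a compute mesh.
; WallWidth, DrawFloor and DrawTop shape that cut to control the walls, floor and top.
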(event EventBeginPlay
  (|CallParentFunction) ; This node is disabled and will not be called.\nDrag off pins to build functionality.
)

(event Collision|EventActorBeginOverlap
  (params (OtherActor :type Actor%20Object%20Reference)))

(event EventTick
  (params (DeltaSeconds :type Float%20%28single-precision%29)))

(event EventOnCreateDynamicMesh
  (params (Target :type Dynamic%20Mesh%20Object%20Reference))
  (bind _handle (Variables|Settings|GetHandle))
  (bind _wallwidth (Variables|Settings|GetWallWidth))
  (bind _wallwidth_2 (Variables|Settings|GetWallWidth))
  (bind _handle_2 (Variables|Settings|GetHandle))
  (bind (_x _y _z) (Class|KismetMathLibrary|BreakVector3f _handle_2))
  (bind (_x_2 _y_2 _z_2) (Class|KismetMathLibrary|BreakVector3f _handle))
  (bind _returnvalue (/ _handle 2.0))
  (bind _returnvalue_2 (/ _handle_2 2.0))
  (bind _returnvalue_3 (Class|GeometryScriptLibraryMeshPrimitiveFunctions|AppendBox Target (Utilities|Struct|MakeGeometryScriptPrimitiveOptions "PerFace" false "Uniform") (Math|Transform|MakeTransform (Math|Vector|MakeVector (.x _returnvalue_2) (.y _returnvalue_2) 0.0) "0, 0, 0" "1.000000,1.000000,1.000000") _x _y _z 0 0 0 "Base" 0))
  (bind _returnvalue_4 (Class|GeometryScriptLibraryMeshUVFunctions|SetMeshUVsfromBoxProjection :TargetMesh _returnvalue_3 :Debug 0))
  (Rendering|Material|SetMaterial (Variables|Default|GetDynamicMeshComponent) 0 (Variables|Settings|GetMaterial))
  (if (Variables|Settings|GetbHollow)
    (bind _returnvalue_5 (DynamicMeshActor|AllocateComputeMesh))
    (bind _returnvalue_6 (Class|GeometryScriptLibraryMeshPrimitiveFunctions|AppendBox _returnvalue_5 (Utilities|Struct|MakeGeometryScriptPrimitiveOptions "PerFace" false "Uniform") (Math|Transform|MakeTransform (Math|Vector|MakeVector (.x _returnvalue) (.y _returnvalue) (Math|Float|SelectFloat (Variables|Settings|GetWallWidth) 0.0 (Variables|Settings|GetDrawFloor))) "0, 0, 0" "1.000000,1.000000,1.000000") (- _x_2 _wallwidth_2) (- _y_2 _wallwidth_2) (- _z_2 (Math|Float|SelectFloat (Math|Float|SelectFloat (* _wallwidth 2.0) _wallwidth (Variables|Settings|GetDrawFloor)) 0.0 (Variables|Settings|GetDrawTop))) 0 0 0 "Base" 0))
    (GeometryScript|Booleans|ApplyMeshBoolean :TargetMesh _returnvalue_4 :ToolMesh _returnvalue_6 :Operation "Subtract" :Debug 0)))

(fn ConstructionScript
  (|CallParentFunction))