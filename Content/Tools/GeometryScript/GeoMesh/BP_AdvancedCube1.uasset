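; BP_AdvancedCube1 is a Geometry Script mesh actor that, despite its name, generates a pointed cone.
; On dynamic mesh creation it appends the cone to the target mesh, taking base radius and height from the Handle vector's Y and Z, with configurable radial steps.
; A disconnected chain holds an unused box builder with UV projection, material assignment and boolean-subtracted hollow walls with floor and top toggles.
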(event EventBeginPlay
  (|CallParentFunction) ; This node is disabled and will not be called.\nDrag off pins to build functionality.
)

(event Collision|EventActorBeginOverlap
  (params (OtherActor :type Actor%20Object%20Reference)))

(event EventTick
  (params (DeltaSeconds :type Float%20%28single-precision%29)))

(event EventOnCreateDynamicMesh
  (params (Target :type Dynamic%20Mesh%20Object%20Reference))
  (bind _handle (Variables|Settings|GetHandle))
  (Class|GeometryScriptLibraryMeshPrimitiveFunctions|AppendCone :TargetMesh Target :Transform (Math|Transform|MakeTransform "0, 0, 0" "0.000000,0.000000,0.000000" "1.000000,1.000000,1.000000") :BaseRadius (.y _handle) :TopRadius 0.0 :Height (.z _handle) :RadialSteps (Variables|Default|GetRadial%20Steps) :HeightSteps 1 :Debug 0))

(fn ConstructionScript
  (|CallParentFunction))