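; Procedural Geometry Script linear staircase generator, sized by a handle with either a fixed or adaptive step count.
; OnCreateDynamicMesh appends the steps, optionally bevels them, and can build convex-hull collision from an extruded triangle or polygon profile.
; Optional left and right railing walls and handles are boxes plane-cut to the pitch derived from the mesh bounds.
; Stairs, railings and handles get separate material slots.
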(event EventBeginPlay
  (|CallParentFunction) ; This node is disabled and will not be called.\nDrag off pins to build functionality.
)

(event EventOnCreateDynamicMesh
  (params (Target :type Dynamic%20Mesh%20Object%20Reference))
  (bind (_handle_y _polygonvertices) (|GetData_2))
  (bind (_offsetcentery _width _height _depth _numberofsteps) (Utilities|AdaptiveStairInfo))
  (bind (_offsetcentery_2 _width_2 _height_2 _depth_2 _numberofsteps_2) (Utilities|FixedStepInfo))
  (bind _dynamicmeshcomponent (Variables|Default|GetDynamicMeshComponent))
  (bind _boxextent (Collision|GetComponentBounds _dynamicmeshcomponent))
  (switch Utilities|FlowControl|Switch|SwitchonEStairType (Variables|Settings|GetStairType)
    (:NewEnumerator0
      (bind _returnvalue (Class|GeometryScriptLibraryMeshPrimitiveFunctions|AppendLinearStairs :TargetMesh Target :Transform (Math|Transform|MakeTransform (Math|Vector|MakeVector 0.0 _offsetcentery 0.0) "0, 0, 0" "1.000000,1.000000,1.000000") :StepWidth _width :StepHeight _height :StepDepth _depth :NumSteps _numberofsteps :bFloating (Variables|Settings|GetbFloating) :Debug 0))
      (Variables|Default|SetTarget%20Mesh _returnvalue))
    (:NewEnumerator1
      (bind _returnvalue_2 (Class|GeometryScriptLibraryMeshPrimitiveFunctions|AppendLinearStairs :TargetMesh Target :Transform (Math|Transform|MakeTransform (Math|Vector|MakeVector 0.0 _offsetcentery_2 0.0) "0, 0, 0" "1.000000,1.000000,1.000000") :StepWidth _width_2 :StepHeight _height_2 :StepDepth _depth_2 :NumSteps _numberofsteps_2 :bFloating (Variables|Settings|GetbFloating) :Debug 0))
      (Variables|Default|SetTarget%20Mesh _returnvalue_2)))
  (if (Variables|Settings|GetbBevel)
    ;[1 1 1] Bevel
    (Class|GeometryScriptLibraryMeshPolygroupFunctions|ComputePolygroupsfromAngleThreshold :TargetMesh (Variables|Default|GetTarget%20Mesh) :CreaseAngle 25.0 :Debug 0)
    (bind _returnvalue_3 (Class|GeometryScriptLibraryMeshModelingFunctions|ApplyMeshPolygroupBevel (Variables|Default|GetTarget%20Mesh) (Utilities|Struct|MakeGeometryScriptMeshBevelOptions (Variables|Settings|GetDistanceBevel) true 0 false "(Min=(X=0.000000,Y=0.000000,Z=0.000000),Max=(X=0.000000,Y=0.000000,Z=0.000000),IsValid=0)" "0.000000,0.000000,0.000000|0.000000,0.000000,-0.000000|1.000000,1.000000,1.000000" true) 0))
    (bind _returnvalue_4 (Class|GeometryScriptLibraryMeshNormalsFunctions|ComputeSplitNormals :TargetMesh _returnvalue_3 :SplitOptions (Utilities|Struct|MakeGeometryScriptSplitNormalsOptions true 25.0 false "(bDefaultLayer=True,ExtendedLayerIndex=0)") :Debug 0))
    (Variables|Default|SetTarget%20Mesh _returnvalue_4))
  (if (Variables|Settings|GetbSimplifiedCollision)
    ;[1 1 1] Generate Simplified Collision
    (bind _returnvalue_5 (DynamicMeshActor|AllocateComputeMesh))
    (bind _output_get (Variables|Default|SetSimplifiedMesh _returnvalue_5))
    (bind _returnvalue_6 (Class|GeometryScriptLibraryMeshPrimitiveFunctions|AppendSimpleExtrudePolygon :TargetMesh _output_get :Transform (Math|Transform|MakeTransform "0, 0, 0" "90.000000,0.000000,90.000000" "1.000000,1.000000,1.000000") :PolygonVertices (select (Variables|Settings|GetbTriangle) (|GetDataTriangle_2) _polygonvertices) :Height _handle_y :Debug 0))
    (bind _output_get_2 (Variables|Default|SetSimplifiedMesh _returnvalue_6))
    (bind _returnvalue_7 (Class|GeometryScriptLibraryCollisionFunctions|SetDynamicMeshCollisionfromMesh _output_get_2 (Variables|Default|GetDynamicMeshComponent) (Utilities|Struct|MakeGeometryScriptCollisionfromMeshOptions false "ConvexHulls" false false false 1.0 false 25 1 0.5 0.0 0.1 0.1 "Z" false 0) 0))
    (Variables|Default|SetTarget%20Mesh _returnvalue_7)
    (else
      ;[1 1 1] Do Not Simplify Collision
      (Class|GeometryScriptLibraryCollisionFunctions|ResetDynamicMeshCollision (Variables|Default|GetDynamicMeshComponent) false 0)))
  (CallFunction|CleanDegenerateTris (Variables|Default|GetTarget%20Mesh) 0.0005 false true)
  (DynamicMeshActor|ReleaseAllComputeMeshes)
  ;[1 1 1] Get the angle for railing
  (Variables|Default|SetRailingCutterAngle (.pitch (Math|Rotator|FindRelativeLookatRotation (Math|Transform|MakeTransform "0, 0, 0" "0, 0, 0" "1.000000,1.000000,1.000000") (Math|Vector|MakeVector (.x _boxextent) 0.0 (.z _boxextent)))))
  ;[1 1 1] Get the bounds of the staircase
  (Variables|Default|SetStairsBounds (.max (Class|GeometryScriptLibraryMeshQueryFunctions|GetMeshBoundingBox (Variables|Default|GetTarget%20Mesh))))
  (Utilities|FlowControl|Sequence
    (:then_0
      (if (Variables|Settings|Railing|GetbMakeLeftRailing)
        ;[1 1 1] Make Left wall
        (bind _returnvalue_8 (DynamicMeshActor|AllocateComputeMesh))
        (bind _returnvalue_9 (Class|GeometryScriptLibraryMeshPrimitiveFunctions|AppendBox :TargetMesh _returnvalue_8 :DimensionX (.x (Variables|Default|GetStairsBounds)) :DimensionY (Variables|Settings|Railing|GetRailingWallWidth) :DimensionZ (* (.z (Variables|Default|GetStairsBounds)) 2.0) :Debug 0))
        (bind _returnvalue_10 (Class|GeometryScriptLibraryMeshBooleanFunctions|ApplyMeshPlaneCut :TargetMesh _returnvalue_9 :CutFrame (Math|Transform|MakeTransform (Math|Vector|MakeVector 0.0 0.0 (+ (/ (.z (Variables|Default|GetStairsBounds)) 2.0) (Variables|Settings|Railing|GetRailingWallHeight))) (Math|Rotator|MakeRotator 0.0 (Variables|Default|GetRailingCutterAngle) 0.0) "1.000000,1.000000,1.000000") :Debug 0))
        (bind _returnvalue_11 (Class|GeometryScriptLibraryMeshBooleanFunctions|ApplyMeshPlaneCut :TargetMesh _returnvalue_10 :CutFrame (Math|Transform|MakeTransform (Math|Vector|MakeVector 0.0 0.0 (/ (.z (Variables|Default|GetStairsBounds)) 2.0)) (Math|Rotator|MakeRotator 0.0 (+ (Variables|Default|GetRailingCutterAngle) 1.8e+02) 0.0) "1.000000,1.000000,1.000000") :Debug 0))
        (bind _returnvalue_12 (GeometryScript|Materials|RemapMaterialIDs _returnvalue_11 0 1 0))
        (bind _returnvalue_13 (GeometryScript|MeshEdits|AppendMesh (Variables|Default|GetTarget%20Mesh) _returnvalue_12 (Math|Transform|MakeTransform (Math|Vector|MakeVector (/ (.x (Variables|Default|GetStairsBounds)) 2.0) (+ (/ (Variables|Settings|Railing|GetRailingWallWidth) 2.0) 1.0) 0.0) "0, 0, 0" "1.000000,1.000000,1.000000") false "(CombineMode=EnableAllMatching)" 0))
        (Variables|Default|SetTarget%20Mesh _returnvalue_13)
        ;[1 1 1] make left railing handle
        (bind _returnvalue_14 (DynamicMeshActor|AllocateComputeMesh))
        (bind _returnvalue_15 (Class|GeometryScriptLibraryMeshPrimitiveFunctions|AppendBox :TargetMesh _returnvalue_14 :DimensionX (* (.x (Variables|Default|GetStairsBounds)) 1.05) :DimensionY (Variables|Settings|Railing|GetRailingTopperDimension) :DimensionZ (* (.z (Variables|Default|GetStairsBounds)) 2.0) :Debug 0))
        (bind _returnvalue_16 (Class|GeometryScriptLibraryMeshBooleanFunctions|ApplyMeshPlaneCut :TargetMesh _returnvalue_15 :CutFrame (Math|Transform|MakeTransform (Math|Vector|MakeVector 0.0 0.0 (+ (/ (.z (Variables|Default|GetStairsBounds)) 2.0) (/ (Variables|Settings|Railing|GetRailingWallHeight) 2.0) (Variables|Settings|Railing|GetRailingTopperDimension))) (Math|Rotator|MakeRotator 0.0 (Variables|Default|GetRailingCutterAngle) 0.0) "1.000000,1.000000,1.000000") :Debug 0))
        (bind _returnvalue_17 (Class|GeometryScriptLibraryMeshBooleanFunctions|ApplyMeshPlaneCut :TargetMesh _returnvalue_16 :CutFrame (Math|Transform|MakeTransform (Math|Vector|MakeVector 0.0 0.0 (- (+ (/ (.z (Variables|Default|GetStairsBounds)) 2.0) (/ (Variables|Settings|Railing|GetRailingWallHeight) 2.0) (Variables|Settings|Railing|GetRailingTopperDimension)) (Variables|Settings|Railing|GetRailingTopperDimension))) (Math|Rotator|MakeRotator 0.0 (+ (Variables|Default|GetRailingCutterAngle) 1.8e+02) 0.0) "1.000000,1.000000,1.000000") :Debug 0))
        (bind _returnvalue_18 (Class|GeometryScriptLibraryMeshModelingFunctions|ApplyMeshPolygroupBevel _returnvalue_17 (Utilities|Struct|MakeGeometryScriptMeshBevelOptions (Variables|Settings|Railing|GetRailingTopBevelAmount) false 0 false "(Min=(X=0.000000,Y=0.000000,Z=0.000000),Max=(X=0.000000,Y=0.000000,Z=0.000000),IsValid=0)" "0.000000,0.000000,0.000000|0.000000,0.000000,-0.000000|1.000000,1.000000,1.000000" true) 0))
        (bind _returnvalue_19 (Class|GeometryScriptLibraryMeshNormalsFunctions|ComputeSplitNormals :TargetMesh _returnvalue_18 :Debug 0))
        (bind _returnvalue_20 (GeometryScript|Materials|RemapMaterialIDs _returnvalue_19 0 2 0))
        (bind _returnvalue_21 (GeometryScript|MeshEdits|AppendMesh (Variables|Default|GetTarget%20Mesh) _returnvalue_20 (Math|Transform|MakeTransform (Math|Vector|MakeVector (/ (.x (Variables|Default|GetStairsBounds)) 2.0) (+ (/ (Variables|Settings|Railing|GetRailingWallWidth) 2.0) 1.0) (* (Variables|Settings|Railing|GetRailingWallHeight) 0.5)) "0, 0, 0" "1.000000,1.000000,1.000000") false "(CombineMode=EnableAllMatching)" 0))
        (Variables|Default|SetTarget%20Mesh _returnvalue_21)))
    (:then_1
      (if (Variables|Settings|Railing|GetbMakeRightRailing)
        ;[1 1 1] Make Left wall
        (bind _returnvalue_22 (DynamicMeshActor|AllocateComputeMesh))
        (bind _returnvalue_23 (Class|GeometryScriptLibraryMeshPrimitiveFunctions|AppendBox :TargetMesh _returnvalue_22 :DimensionX (.x (Variables|Default|GetStairsBounds)) :DimensionY (Variables|Settings|Railing|GetRailingWallWidth) :DimensionZ (* (.z (Variables|Default|GetStairsBounds)) 2.0) :Debug 0))
        (bind _returnvalue_24 (Class|GeometryScriptLibraryMeshBooleanFunctions|ApplyMeshPlaneCut :TargetMesh _returnvalue_23 :CutFrame (Math|Transform|MakeTransform (Math|Vector|MakeVector 0.0 0.0 (+ (/ (.z (Variables|Default|GetStairsBounds)) 2.0) (Variables|Settings|Railing|GetRailingWallHeight))) (Math|Rotator|MakeRotator 0.0 (Variables|Default|GetRailingCutterAngle) 0.0) "1.000000,1.000000,1.000000") :Debug 0))
        (bind _returnvalue_25 (Class|GeometryScriptLibraryMeshBooleanFunctions|ApplyMeshPlaneCut :TargetMesh _returnvalue_24 :CutFrame (Math|Transform|MakeTransform (Math|Vector|MakeVector 0.0 0.0 (/ (.z (Variables|Default|GetStairsBounds)) 2.0)) (Math|Rotator|MakeRotator 0.0 (+ (Variables|Default|GetRailingCutterAngle) 1.8e+02) 0.0) "1.000000,1.000000,1.000000") :Debug 0))
        (bind _returnvalue_26 (GeometryScript|Materials|RemapMaterialIDs _returnvalue_25 0 1 0))
        (bind _returnvalue_27 (GeometryScript|MeshEdits|AppendMesh (Variables|Default|GetTarget%20Mesh) _returnvalue_26 (Math|Transform|MakeTransform (Math|Vector|MakeVector (/ (.x (Variables|Default|GetStairsBounds)) 2.0) (- (.y (Variables|Default|GetStairsBounds)) (+ (/ (Variables|Settings|Railing|GetRailingWallWidth) 2.0) 1.0)) 0.0) "0, 0, 0" "1.000000,1.000000,1.000000") false "(CombineMode=EnableAllMatching)" 0))
        (Variables|Default|SetTarget%20Mesh _returnvalue_27)
        ;[1 1 1] make left railing handle
        (bind _returnvalue_28 (DynamicMeshActor|AllocateComputeMesh))
        (bind _returnvalue_29 (Class|GeometryScriptLibraryMeshPrimitiveFunctions|AppendBox :TargetMesh _returnvalue_28 :DimensionX (* (.x (Variables|Default|GetStairsBounds)) 1.05) :DimensionY (Variables|Settings|Railing|GetRailingTopperDimension) :DimensionZ (* (.z (Variables|Default|GetStairsBounds)) 2.0) :Debug 0))
        (bind _returnvalue_30 (Class|GeometryScriptLibraryMeshBooleanFunctions|ApplyMeshPlaneCut :TargetMesh _returnvalue_29 :CutFrame (Math|Transform|MakeTransform (Math|Vector|MakeVector 0.0 0.0 (+ (/ (.z (Variables|Default|GetStairsBounds)) 2.0) (/ (Variables|Settings|Railing|GetRailingWallHeight) 2.0) (Variables|Settings|Railing|GetRailingTopperDimension))) (Math|Rotator|MakeRotator 0.0 (Variables|Default|GetRailingCutterAngle) 0.0) "1.000000,1.000000,1.000000") :Debug 0))
        (bind _returnvalue_31 (Class|GeometryScriptLibraryMeshBooleanFunctions|ApplyMeshPlaneCut :TargetMesh _returnvalue_30 :CutFrame (Math|Transform|MakeTransform (Math|Vector|MakeVector 0.0 0.0 (- (+ (/ (.z (Variables|Default|GetStairsBounds)) 2.0) (/ (Variables|Settings|Railing|GetRailingWallHeight) 2.0) (Variables|Settings|Railing|GetRailingTopperDimension)) (Variables|Settings|Railing|GetRailingTopperDimension))) (Math|Rotator|MakeRotator 0.0 (+ (Variables|Default|GetRailingCutterAngle) 1.8e+02) 0.0) "1.000000,1.000000,1.000000") :Debug 0))
        (bind _returnvalue_32 (Class|GeometryScriptLibraryMeshModelingFunctions|ApplyMeshPolygroupBevel _returnvalue_31 (Utilities|Struct|MakeGeometryScriptMeshBevelOptions (Variables|Settings|Railing|GetRailingTopBevelAmount) false 0 false "(Min=(X=0.000000,Y=0.000000,Z=0.000000),Max=(X=0.000000,Y=0.000000,Z=0.000000),IsValid=0)" "0.000000,0.000000,0.000000|0.000000,0.000000,-0.000000|1.000000,1.000000,1.000000" true) 0))
        (bind _returnvalue_33 (Class|GeometryScriptLibraryMeshNormalsFunctions|ComputeSplitNormals :TargetMesh _returnvalue_32 :Debug 0))
        (bind _returnvalue_34 (GeometryScript|Materials|RemapMaterialIDs _returnvalue_33 0 2 0))
        (bind _returnvalue_35 (GeometryScript|MeshEdits|AppendMesh (Variables|Default|GetTarget%20Mesh) _returnvalue_34 (Math|Transform|MakeTransform (Math|Vector|MakeVector (/ (.x (Variables|Default|GetStairsBounds)) 2.0) (- (.y (Variables|Default|GetStairsBounds)) (+ (/ (Variables|Settings|Railing|GetRailingWallWidth) 2.0) 1.0)) (* (Variables|Settings|Railing|GetRailingWallHeight) 0.5)) "0, 0, 0" "1.000000,1.000000,1.000000") false "(CombineMode=EnableAllMatching)" 0))
        (Variables|Default|SetTarget%20Mesh _returnvalue_35)))
    (:then_2
      ;[1 1 1] Apply Material
      (Class|DynamicMeshComponent|ConfigureMaterialSet (Variables|Default|GetDynamicMeshComponent) (Utilities|Array|MakeArray (Variables|Settings|Materials|GetStairsMaterial) (Variables|Settings|Materials|GetRailingMaterial) (Variables|Settings|Materials|GetRailingHandleMaterial)))
      (DynamicMeshActor|ReleaseAllComputeMeshes))))

(fn ConstructionScript
  (|CallParentFunction))