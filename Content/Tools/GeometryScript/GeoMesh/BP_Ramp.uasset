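; BP_Ramp is a Geometry Script generated-mesh actor that builds a parametric ramp from TopPoint and FloorPoint.
; On mesh creation it triangulates a four-point side profile, rotated upright, then linearly extrudes it along Y by TopPoint.Y to set the width.
; It then cleans degenerate triangles, applies the Material, releases compute meshes and enables complex-as-simple collision so the collision follows the generated shape.
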(event EventBeginPlay
  (|CallParentFunction) ; This node is disabled and will not be called.\nDrag off pins to build functionality.
)

(event Collision|EventActorBeginOverlap
  (params (OtherActor :type Actor%20Object%20Reference)))

(event EventTick
  (params (DeltaSeconds :type Float%20%28single-precision%29)))

(event EventOnCreateDynamicMesh
  (params (Target :type Dynamic%20Mesh%20Object%20Reference))
  (bind _toppoint (Variables|Settings|GetTopPoint))
  (bind _dynamicmeshcomponent (Variables|Default|GetDynamicMeshComponent))
  (bind _returnvalue (Class|GeometryScriptLibraryMeshPrimitiveFunctions|AppendTriangulatedPolygon :TargetMesh Target :Transform (Math|Transform|MakeTransform (Math|Vector|MakeVector 0.0 0.0 (.z _toppoint)) "0.000000,0.000000,90.000000" "1.000000,1.000000,1.000000") :PolygonVertices (Utilities|Array|MakeArray "" (Math|Vector2D|MakeVector2D 0.0 (.z _toppoint)) (Math|Vector2D|MakeVector2D (.x (Variables|Settings|GetFloorPoint)) (.z _toppoint)) (Math|Vector2D|MakeVector2D (.x _toppoint) 0.0)) :Debug 0))
  (bind _returnvalue_2 (Class|GeometryScriptLibraryMeshModelingFunctions|ApplyMeshLinearExtrudeFaces :TargetMesh _returnvalue :Options (Utilities|Struct|MakeGeometryScriptMeshLinearExtrudeOptions (.y _toppoint) "FixedDirection" (Math|Vector|MakeVector 0.0 1.0 0.0) "EntireSelection" "(GroupMode=PreserveExisting,ConstantGroup=0)" 1.0 true) :Debug 0))
  (CallFunction|CleanDegenerateTris _returnvalue_2 0.0005 false true)
  (Class|DynamicMeshComponent|ConfigureMaterialSet _dynamicmeshcomponent (Utilities|Array|MakeArray (Variables|Settings|GetMaterial)))
  (DynamicMeshActor|ReleaseAllComputeMeshes)
  (Class|DynamicMeshComponent|EnableComplexasSimpleCollision _dynamicmeshcomponent))

(fn ConstructionScript
  (|CallParentFunction))