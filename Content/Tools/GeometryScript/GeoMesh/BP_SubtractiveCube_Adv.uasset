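; BP_SubtractiveCube_Adv is a Geometry Script tool actor that supplies a box as a subtractive shape for mesh generation.
; The construction script fits the Cube between the actor origin and the Handle vector, centering it at half the vector and scaling it from the absolute value.
; ShowDebug toggles the cube's visibility.
; GetGeometrySubtractiveComponents returns the Cube as the component to subtract.
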(event EventBeginPlay
  (|CallParentFunction) ; This node is disabled and will not be called.\nDrag off pins to build functionality.
)

(event Collision|EventActorBeginOverlap
  (params (OtherActor :type Actor%20Object%20Reference))
  (|CallParentFunction OtherActor) ; This node is disabled and will not be called.\nDrag off pins to build functionality.
)

(event EventTick
  (params (DeltaSeconds :type Float%20%28single-precision%29))
  (|CallParentFunction DeltaSeconds) ; This node is disabled and will not be called.\nDrag off pins to build functionality.
)

(fn ConstructionScript
  (bind _cube (Variables|Default|GetCube))
  (bind _cube_2 (Variables|Default|GetCube))
  (|CallParentFunction)
  (Utilities|FlowControl|Sequence
    (:then_0
      (if (Variables|Settings|GetShowDebug)
        (Rendering|SetVisibility _cube_2 true false)
        (else
          (Rendering|SetVisibility _cube_2 false false))))
    (:then_1
      (Transformation|SetRelativeLocation _cube (/ (Variables|Settings|GetHandle) (Math|Float|MakeLiteralFloat 2.0)) false false)
      (Transformation|SetRelativeScale3D _cube (/ (Math|Vector|VectorGetAbs (Variables|Settings|GetHandle)) (Math|Float|MakeLiteralFloat 1e+02))))))

(fn GetGeometrySubtractiveComponents
  (return (Utilities|Array|MakeArray (Variables|Default|GetCube))))