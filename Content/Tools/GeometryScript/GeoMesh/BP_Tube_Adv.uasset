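; Geometry Script tool actor that generates a parametric tube or arced wall, with optional bevel, gapped repeated segments and cut-out windows.
; Construction script constrains handle vectors that size the rectangular profile, which is revolved and repeated by yaw rotation.
; WindowCutter extrudes rounded rectangles, optionally repeats them, and boolean-subtracts them, or unions them in a debug material for preview.
; Split normals, degenerate-triangle cleanup and material assignment finish the mesh.
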(event EventBeginPlay
  (|CallParentFunction) ; This node is disabled and will not be called.\nDrag off pins to build functionality.
)

(event EventOnCreateDynamicMesh
  (params (Target :type Dynamic%20Mesh%20Object%20Reference))
  ;[1 1 1] Create Tube
  (bind _returnvalue (Class|GeometryScriptLibraryMeshPrimitiveFunctions|AppendRevolvePolygon :TargetMesh Target :PolygonVertices (|MakePolygonVertices) :RevolveOptions (|GetRevolveOptions_2) :Radius (|GetRadius) :Steps (Variables|Settings|Revolve|GetSteps) :Debug 0))
  (Variables|Default|SetDynamicMesh _returnvalue)
  (if (Variables|Settings|Bevel|GetbBevel)
    ;[1 1 1] Bevel
    (bind _returnvalue_2 (Class|GeometryScriptLibraryMeshModelingFunctions|ApplyMeshPolygroupBevel (Variables|Default|GetDynamicMesh) (Utilities|Struct|MakeGeometryScriptMeshBevelOptions (Variables|Settings|Bevel|GetBevelDistance) false 0 false "(Min=(X=0.000000,Y=0.000000,Z=0.000000),Max=(X=0.000000,Y=0.000000,Z=0.000000),IsValid=0)" "0.000000,0.000000,0.000000|0.000000,0.000000,-0.000000|1.000000,1.000000,1.000000" true) 0))
    (Variables|Default|SetDynamicMesh _returnvalue_2))
  (if (Variables|Settings|Repeater|GetbRepeaterWall)
    (CallFunction|FnRepeater (Variables|Default|GetDynamicMesh) (Variables|Settings|Repeater|GetInstances)))
  (DynamicMeshActor|ReleaseAllComputeMeshes)
  (if (Variables|Settings|Window|GetbWindow)
    (Utilities|WindowCutter))
  ;[1 1 1] This helps smoothing the Normals
  (Class|GeometryScriptLibraryMeshNormalsFunctions|ComputeSplitNormals :TargetMesh (Variables|Default|GetDynamicMesh) :SplitOptions (Utilities|Struct|MakeGeometryScriptSplitNormalsOptions true 45.0 false "(bDefaultLayer=True,ExtendedLayerIndex=0)") :Debug 0)
  ;[1 1 1] Apply Materials
  (CallFunction|CleanDegenerateTris 0 0.0005 false true)
  (Class|DynamicMeshComponent|ConfigureMaterialSet (Variables|Default|GetDynamicMeshComponent) (Utilities|Array|MakeArray (Variables|Settings|Revolve|GetMaterial) "/Game/Tools/OldGeo/Materials/MT_DebugTool.MT_DebugTool")))

(fn ConstructionScript
  (bind _returnvalue (Math|Float|Clamp(Float) 0.0 0.0 0.0))
  (|CallParentFunction)
  (Variables|Settings|SetVectorHandle (Math|Vector|MakeVector (Math|Float|Max(Float) (.x (Variables|Settings|GetVectorHandle)) 0.0) (Math|Float|Clamp(Float) (.y (Variables|Settings|GetVectorHandle)) 0.0 0.0) (Math|Float|Max(Float) (.z (Variables|Settings|GetVectorHandle)) 0.0)))
  (Variables|Settings|SetThicknessHandle (Math|Vector|MakeVector (Math|Float|Max(Float) (.x (Variables|Settings|GetThicknessHandle)) (.x (Variables|Settings|GetVectorHandle))) _returnvalue _returnvalue))
  (bind _output_get (Variables|Settings|SetWindowHandle (Math|Vector|MakeVector 0.0 0.0 (.z (Variables|Settings|GetWindowHandle)))))
  (Variables|Settings|Window|SetHeight (.z _output_get)))

(fn FnRepeater
  (params (InMesh :type Dynamic%20Mesh%20Object%20Reference) (Instances :type Integer))
  (bind _returnvalue (DynamicMeshActor|AllocateComputeMesh))
  (bind _copytomeshout (GeometryScript|Decomposition|CopyMeshtoMesh InMesh _returnvalue 0))
  (bind _returnvalue_2 (Class|GeometryScriptLibraryMeshBasicEditFunctions|AppendMeshRepeated InMesh _copytomeshout (Math|Transform|MakeTransform "0, 0, 0" (Math|Rotator|MakeRotator 0.0 0.0 (|GetRotationRate_2)) "1.000000,1.000000,1.000000") (- Instances 1) true false "(CombineMode=EnableAllMatching)" 0))
  (return _returnvalue_2))