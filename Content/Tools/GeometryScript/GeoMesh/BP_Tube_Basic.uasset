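; BP_Tube_Basic is a Geometry Script tool actor that generates a parametric tube mesh with adjustable sweep angle and step count.
; Two vector handles drive its shape: VectorHandle sets inner radius and height, and ThicknessHandle sets wall thickness, with the construction script constraining both.
; OnCreateDynamicMesh revolves a rectangular profile from these handles, optionally bevels polygroups, cleans degenerate triangles and applies the material.
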(event EventBeginPlay
  (|CallParentFunction) ; This node is disabled and will not be called.\nDrag off pins to build functionality.
)

(event EventOnCreateDynamicMesh
  (params (Target :type Dynamic%20Mesh%20Object%20Reference))
  (bind _returnvalue (Transformation|GetActorLocation))
  (bind _vectorhandle (Variables|Settings|GetVectorHandle))
  (bind _thicknesshandle (Variables|Settings|GetThicknessHandle))
  (bind _vectorhandle_2 (Variables|Settings|GetVectorHandle))
  (bind _returnvalue_2 (Math|Vector|Distance2D(Vector) _vectorhandle _thicknesshandle))
  ;[1 1 1] Tube Generation
  (bind _returnvalue_3 (Class|GeometryScriptLibraryMeshPrimitiveFunctions|AppendRevolvePolygon :TargetMesh Target :PolygonVertices (Utilities|Array|MakeArray "(X=0.000000,Y=0.000000)" (Math|Vector2D|MakeVector2D _returnvalue_2 0.0) (Math|Vector2D|MakeVector2D _returnvalue_2 (.z _vectorhandle_2)) (Math|Vector2D|MakeVector2D 0.0 (.z _vectorhandle_2))) :RevolveOptions (Utilities|Struct|MakeGeometryScriptRevolveOptions (Variables|Settings|GetRevolve%20Degrees) (Variables|Settings|GetStartOffset) false true) :Radius (Math|Float|Absolute(Float) (Math|Vector|Distance2D(Vector) (+ (Variables|Settings|GetVectorHandle) _returnvalue) _returnvalue)) :Steps (Variables|Settings|GetSteps) :Debug 0))
  (Variables|Default|SetTarget%20Mesh _returnvalue_3)
  (if (Variables|Settings|GetbBevel)
    ;[1 1 1] Bevel
    (bind _returnvalue_4 (Class|GeometryScriptLibraryMeshModelingFunctions|ApplyMeshPolygroupBevel (Variables|Default|GetTarget%20Mesh) (Utilities|Struct|MakeGeometryScriptMeshBevelOptions (Variables|Settings|GetBevelDistance) false 0 false "(Min=(X=0.000000,Y=0.000000,Z=0.000000),Max=(X=0.000000,Y=0.000000,Z=0.000000),IsValid=0)" "0.000000,0.000000,0.000000|0.000000,0.000000,-0.000000|1.000000,1.000000,1.000000" true) 0))
    (Variables|Default|SetTarget%20Mesh _returnvalue_4))
  ;[1 1 1] Apply Material
  (CallFunction|CleanDegenerateTris (Variables|Default|GetTarget%20Mesh) 0.0005 false true)
  (Class|DynamicMeshComponent|ConfigureMaterialSet (Variables|Default|GetDynamicMeshComponent) (Utilities|Array|MakeArray (Variables|Settings|GetMaterial))))

(fn ConstructionScript
  (bind _returnvalue (Math|Float|Clamp(Float) 0.0 0.0 0.0))
  (|CallParentFunction)
  (Variables|Settings|SetVectorHandle (Math|Vector|MakeVector (Math|Float|Max(Float) (.x (Variables|Settings|GetVectorHandle)) 0.0) (Math|Float|Clamp(Float) (.y (Variables|Settings|GetVectorHandle)) 0.0 0.0) (Math|Float|Max(Float) (.z (Variables|Settings|GetVectorHandle)) 0.0)))
  (Variables|Settings|SetThicknessHandle (Math|Vector|MakeVector (Math|Float|Max(Float) (.x (Variables|Settings|GetThicknessHandle)) (.x (Variables|Settings|GetVectorHandle))) _returnvalue _returnvalue)))